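; BP_TemperatureManager is a manager actor that gives scene meshes random stand-in temperatures through custom depth stencil values.
; On BeginPlay, and again on pressing A, it scans all actors, enabling custom depth with random stencils on static and dynamic mesh components.
; It disables their shadows, which read hotter under an invert filter.
; The dynamic mesh pass is nested in the static mesh loop, so it skips actors without static meshes.
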(event EventBeginPlay
  (bind _returnvalue (Math|Random|RandomInteger 255))
  (Input|EnableInput (Game|GetPlayerController 0))
  (bind _outactors (Actor|GetAllActorsOfClass "/Script/Engine.Actor"))
  (for (_array_element _array_index) _outactors
    (for _array_element_2 (Actor|GetComponentsByClass _array_element "/Script/Engine.StaticMeshComponent")
      (Rendering|SetRenderCustomDepth _array_element_2 true)
      (Rendering|SetCustomDepthStencilValue _array_element_2 _returnvalue)
      ;[1 1 1] hide shadows cus they turn up hotter due to the invert filter
      (Rendering|SetCastShadow _array_element_2 false)
      (for _array_element_3 (Actor|GetComponentsByClass _array_element "/Script/GeometryFramework.DynamicMeshComponent")
        (Rendering|SetRenderCustomDepth _array_element_3 true)
        (Rendering|SetCustomDepthStencilValue _array_element_3 _returnvalue)
        (Rendering|SetCastShadow _array_element_3 false)))))

(event Collision|EventActorBeginOverlap
  (params (OtherActor :type Actor%20Object%20Reference)))

(event EventTick
  (params (DeltaSeconds :type Float%20%28single-precision%29)))

(event Input|KeyboardEvents|A
  (params (Key :type Key%20Structure :default "None"))
  (bind _returnvalue (Math|Random|RandomInteger 255))
  (:Pressed
    (bind _outactors (Actor|GetAllActorsOfClass "/Script/Engine.Actor"))
    (for (_array_element _array_index) _outactors
      (for _array_element_2 (Actor|GetComponentsByClass _array_element "/Script/Engine.StaticMeshComponent")
        (Rendering|SetRenderCustomDepth _array_element_2 true)
        (Rendering|SetCustomDepthStencilValue _array_element_2 _returnvalue)
        ;[1 1 1] hide shadows cus they turn up hotter due to the invert filter
        (Rendering|SetCastShadow _array_element_2 false)
        (for _array_element_3 (Actor|GetComponentsByClass _array_element "/Script/GeometryFramework.DynamicMeshComponent")
          (Rendering|SetRenderCustomDepth _array_element_3 true)
          (Rendering|SetCustomDepthStencilValue _array_element_3 _returnvalue)
          (Rendering|SetCastShadow _array_element_3 false))))))

(fn ConstructionScript)